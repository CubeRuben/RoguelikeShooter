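; Turret actor Blueprint that adds firing sounds and death effects to an enum-driven hitscan or projectile attack.
; On each shot it plays a rifle or rocket sound to match the attack type.
; When destroyed, the authority spawns a damaging explosion, then rolls for a health or random ammo pickup.
; If that roll fails, a second chance roll can drop a firearm pickup built from a random definition.
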(event EventDestroyed
  (bind _returnvalue (Transformation|GetActorLocation))
  (bind _ammodef (Variables|Default|GetAmmoDef))
  (bind _firearmdef (Variables|Default|GetFirearmDef))
  (bind _returnvalue_2 (+ _returnvalue "0.000000,0.000000,50.000000"))
  (Networking|SwitchHasAuthority
    (:Authority
      (bind _returnvalue_3 (Game|SpawnActorfromClass "/Script/RoguelikeShooter.Explosion" (Math|Transform|MakeTransform (Transformation|GetActorLocation) "0, 0, 0" "1.000000,1.000000,1.000000") "AlwaysSpawn" "MultiplyWithRoot" 0 0))
      (Utilities|IsValid _returnvalue_3
        (:Is%20Valid
          (Class|Explosion|InitExplosion _returnvalue_3 self 25.0 5e+02 2e+05))
        (:Is%20Not%20Valid
          _))
      (if (< (Math|Random|RandomFloat) (Variables|Default|GetPickupChance))
        (if (Math|Random|RandomBool)
          (Game|SpawnActorfromClass "/Game/Blueprint/BP_HalthPackPickup.BP_HalthPackPickup_C" (Math|Transform|MakeTransform _returnvalue_2 "0, 0, 0" "1.000000,1.000000,1.000000") "Undefined" "MultiplyWithRoot" 0 0)
          (else
            (bind _returnvalue_4 (Game|SpawnActorfromClass "/Game/Blueprint/BP_AmmoPickup.BP_AmmoPickup_C" (Math|Transform|MakeTransform _returnvalue_2 "0, 0, 0" "1.000000,1.000000,1.000000") "Undefined" "MultiplyWithRoot" 0 0))
            (Utilities|IsValid _returnvalue_4
              (:Is%20Valid
                (Default|Init _returnvalue_4 (Utilities|Array|Get(acopy) _ammodef (Math|Random|RandomInteger (Utilities|Array|Length _ammodef))))))))
        (elif (< (Math|Random|RandomFloat) (Variables|Default|GetFirearmChance))
          (bind _returnvalue_5 (Game|SpawnActorfromClass "/Script/RoguelikeShooter.FirearmPickup" (Math|Transform|MakeTransform _returnvalue_2 "0, 0, 0" "1.000000,1.000000,1.000000") "AlwaysSpawn" "MultiplyWithRoot" 0 0))
          (Utilities|IsValid _returnvalue_5
            (:Is%20Valid
              (bind _returnvalue_6 (Game|ConstructObjectfromClass "/Script/RoguelikeShooter.Firearm"))
              (Class|Firearm|SetFirearmDefinition _returnvalue_6 (Utilities|Array|Get(acopy) _firearmdef (Math|Random|RandomInteger (Utilities|Array|Length _firearmdef))))
              (Class|FirearmPickup|SetFirearm _returnvalue_5 _returnvalue_6))))))))

(event EventOnShot
  (bind _returnvalue (Transformation|GetActorLocation))
  (switch Utilities|FlowControl|Switch|SwitchonETurretAttackType (Variables|Default|GetAttackType)
    (:Hitscan
      (Audio|PlaySoundatLocation "/Game/SFX/Firearms/Rifle/SC_RifleShot.SC_RifleShot" _returnvalue "0, 0, 0" 1.0 1.0 0.0 0 0 0 0))
    (:Projectile
      (Audio|PlaySoundatLocation "/Game/SFX/Firearms/RPG/SC_Rocket.SC_Rocket" _returnvalue "0, 0, 0" 1.0 1.0 0.0 0 0 0 0))))

(fn ConstructionScript)