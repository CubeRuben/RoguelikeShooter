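; BP_AmmoPickup is an ammo pickup actor configured by an AmmoDefinition asset.
; The Construction Script shows the definition's name on a TextRender and sets AmmoAmount to a rounded quarter of its MaxAmount.
; Without a valid definition, it clears the text and zeroes the amount.
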(fn ConstructionScript
  (bind _textrender (Variables|Default|GetTextRender))
  (Utilities|IsValid (Variables|Default|GetAmmoDefinition)
    (:Is%20Valid
      (Rendering|Components|TextRender|SetText _textrender (Utilities|Text|ToText(String) (Variables|/Script/RoguelikeShooter.AmmoDefinition|GetName (Variables|Default|GetAmmoDefinition))))
      (Variables|Default|SetAmmoAmount (Math|Float|Round (/ (Variables|/Script/RoguelikeShooter.AmmoDefinition|GetMaxAmount (Variables|Default|GetAmmoDefinition)) 4))))
    (:Is%20Not%20Valid
      (Rendering|Components|TextRender|SetText _textrender (Utilities|Text|MakeLiteralText ""))
      (Variables|Default|SetAmmoAmount 0))))