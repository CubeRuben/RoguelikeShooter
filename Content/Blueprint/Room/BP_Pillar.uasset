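; Procedurally built pillar actor that stacks random plain or doorway segments, with platforms spawned at the doorways.
; A seeded random stream sets the base yaw in 60-degree steps and picks each segment's mesh by PlatformChance, rotating segments progressively up the stack.
; Init stores the seed and builds, while remote instances build on BeginPlay from their Seed value.
; Only the authority spawns the platform variations, initializing each with a number from the stream.
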(event Custom|Init
  (params (Seed :type Integer))
  (bind _platformvariations (Variables|Default|GetPlatformVariations))
  (Variables|Default|SetSeed Seed)
  (Variables|Default|SetRandom%20Stream (Math|Random|MakeRandomStream (Variables|Default|GetSeed)))
  (Transformation|SetActorRotation (Math|Rotator|MakeRotator 0.0 0.0 (* (Class|KismetMathLibrary|RandomIntegerfromStream (Variables|Default|GetRandom%20Stream) 6) 6e+01)))
  (for _index (range 1 5)
    (bind _returnvalue (AddComponent|AddStaticMeshComponent true (Math|Transform|MakeTransform (Math|Vector|MakeVector 0.0 0.0 (* _index 6e+02)) (Math|Rotator|MakeRotator 0.0 0.0 (* _index 60)) "1.000000,1.000000,1.000000")))
    (Transformation|AttachComponentToComponent _returnvalue (Variables|Default|GetDefaultSceneRoot) "None" "KeepRelative" "KeepRelative" "KeepRelative" true)
    (if (> (Variables|Default|GetPlatformChance) (Math|Random|RandomFloatfromStream (Variables|Default|GetRandom%20Stream)))
      (Components|StaticMesh|SetStaticMesh _returnvalue "/Game/Meshes/Room/SM_PillarDoorway.SM_PillarDoorway")
      (Networking|SwitchHasAuthority
        (:Authority
          (bind _returnvalue_2 (Game|SpawnActorfromClass (Utilities|Array|Get(acopy) _platformvariations (Class|KismetMathLibrary|RandomIntegerfromStream (Variables|Default|GetRandom%20Stream) (Utilities|Array|Length _platformvariations))) (Math|Transform|MakeTransform (Transformation|GetWorldLocation _returnvalue) "0, 0, 0" "1.000000,1.000000,1.000000") "Undefined" "MultiplyWithRoot" 0 0))
          (Default|Init _returnvalue_2 (Class|KismetMathLibrary|RandomIntegerfromStream (Variables|Default|GetRandom%20Stream) 2500))))
      (else
        (Components|StaticMesh|SetStaticMesh _returnvalue "/Game/Meshes/Room/SM_Pillar.SM_Pillar")))))

(event EventBeginPlay
  (bind _platformvariations (Variables|Default|GetPlatformVariations))
  (Networking|SwitchHasAuthority
    (:Remote
      (Variables|Default|SetRandom%20Stream (Math|Random|MakeRandomStream (Variables|Default|GetSeed)))
      (Transformation|SetActorRotation (Math|Rotator|MakeRotator 0.0 0.0 (* (Class|KismetMathLibrary|RandomIntegerfromStream (Variables|Default|GetRandom%20Stream) 6) 6e+01)))
      (for _index (range 1 5)
        (bind _returnvalue (AddComponent|AddStaticMeshComponent true (Math|Transform|MakeTransform (Math|Vector|MakeVector 0.0 0.0 (* _index 6e+02)) (Math|Rotator|MakeRotator 0.0 0.0 (* _index 60)) "1.000000,1.000000,1.000000")))
        (Transformation|AttachComponentToComponent _returnvalue (Variables|Default|GetDefaultSceneRoot) "None" "KeepRelative" "KeepRelative" "KeepRelative" true)
        (if (> (Variables|Default|GetPlatformChance) (Math|Random|RandomFloatfromStream (Variables|Default|GetRandom%20Stream)))
          (Components|StaticMesh|SetStaticMesh _returnvalue "/Game/Meshes/Room/SM_PillarDoorway.SM_PillarDoorway")
          (Networking|SwitchHasAuthority
            (:Authority
              (bind _returnvalue_2 (Game|SpawnActorfromClass (Utilities|Array|Get(acopy) _platformvariations (Class|KismetMathLibrary|RandomIntegerfromStream (Variables|Default|GetRandom%20Stream) (Utilities|Array|Length _platformvariations))) (Math|Transform|MakeTransform (Transformation|GetWorldLocation _returnvalue) "0, 0, 0" "1.000000,1.000000,1.000000") "Undefined" "MultiplyWithRoot" 0 0))
              (Default|Init _returnvalue_2 (Class|KismetMathLibrary|RandomIntegerfromStream (Variables|Default|GetRandom%20Stream) 2500))))
          (else
            (Components|StaticMesh|SetStaticMesh _returnvalue "/Game/Meshes/Room/SM_Pillar.SM_Pillar")))))))

(fn ConstructionScript)