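; Hexagonal room platform actor that procedurally builds its rotation, walls and bridges from a seed.
; Generation runs from Init(Seed), or on BeginPlay for remote clients, using a seeded random stream for a 60-degree-step yaw and chance-based wall meshes on six sides.
; Only the authority then rolls for bridge actors in six directions, picking random variations and skipping spawns that would collide.
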(event Custom|Init
  (params (Seed :type Integer))
  (bind _bridgevariations (Variables|Default|GetBridgeVariations))
  (bind _output_get (Variables|Default|SetSeed Seed))
  (Variables|Default|SetRandom%20Stream (Math|Random|MakeRandomStream _output_get))
  (Transformation|SetActorRotation (Math|Rotator|MakeRotator 0.0 0.0 (* (Class|KismetMathLibrary|RandomIntegerfromStream (Variables|Default|GetRandom%20Stream) 6) 6e+01)))
  (for _index (range 0 5)
    (if (> (Variables|Default|GetWallChance) (Math|Random|RandomFloatfromStream (Variables|Default|GetRandom%20Stream)))
      (bind _returnvalue (AddComponent|AddStaticMeshComponent true (Math|Transform|MakeTransform "0, 0, 0" (Math|Rotator|MakeRotator 0.0 0.0 (* _index 6e+01)) "1.000000,1.000000,1.000000")))
      (Transformation|AttachComponentToComponent _returnvalue (Variables|Default|GetSM_Platform) "None" "KeepRelative" "KeepRelative" "KeepRelative" true)
      (Components|StaticMesh|SetStaticMesh _returnvalue "/Game/Meshes/Room/SM_PlatformWall.SM_PlatformWall")))
  (Networking|SwitchHasAuthority
    (:Authority
      (for _index_2 (range 0 5)
        (if (> (Variables|Default|GetBridgeChance) (Math|Random|RandomFloatfromStream (Variables|Default|GetRandom%20Stream)))
          (Game|SpawnActorfromClass (Utilities|Array|Get(acopy) _bridgevariations (Class|KismetMathLibrary|RandomIntegerfromStream (Variables|Default|GetRandom%20Stream) (Utilities|Array|Length _bridgevariations))) (Math|Transform|MakeTransform (Transformation|GetWorldLocation (Variables|Default|GetSM_Platform)) (Math|Rotator|MakeRotator 0.0 0.0 (* _index_2 6e+01)) "1.000000,1.000000,1.000000") "DontSpawnIfColliding" "MultiplyWithRoot" 0 0))))))

(event EventTick
  (params (DeltaSeconds :type Float%20%28single-precision%29)))

(event EventBeginPlay
  (bind _bridgevariations (Variables|Default|GetBridgeVariations))
  (Networking|SwitchHasAuthority
    (:Remote
      (Variables|Default|SetRandom%20Stream (Math|Random|MakeRandomStream (stale Custom|Init _output_get)))
      (Transformation|SetActorRotation (Math|Rotator|MakeRotator 0.0 0.0 (* (Class|KismetMathLibrary|RandomIntegerfromStream (Variables|Default|GetRandom%20Stream) 6) 6e+01)))
      (for _index (range 0 5)
        (if (> (Variables|Default|GetWallChance) (Math|Random|RandomFloatfromStream (Variables|Default|GetRandom%20Stream)))
          (bind _returnvalue (AddComponent|AddStaticMeshComponent true (Math|Transform|MakeTransform "0, 0, 0" (Math|Rotator|MakeRotator 0.0 0.0 (* _index 6e+01)) "1.000000,1.000000,1.000000")))
          (Transformation|AttachComponentToComponent _returnvalue (Variables|Default|GetSM_Platform) "None" "KeepRelative" "KeepRelative" "KeepRelative" true)
          (Components|StaticMesh|SetStaticMesh _returnvalue "/Game/Meshes/Room/SM_PlatformWall.SM_PlatformWall")))
      (Networking|SwitchHasAuthority
        (:Authority
          (for _index_2 (range 0 5)
            (if (> (Variables|Default|GetBridgeChance) (Math|Random|RandomFloatfromStream (Variables|Default|GetRandom%20Stream)))
              (Game|SpawnActorfromClass (Utilities|Array|Get(acopy) _bridgevariations (Class|KismetMathLibrary|RandomIntegerfromStream (Variables|Default|GetRandom%20Stream) (Utilities|Array|Length _bridgevariations))) (Math|Transform|MakeTransform (Transformation|GetWorldLocation (Variables|Default|GetSM_Platform)) (Math|Rotator|MakeRotator 0.0 0.0 (* _index_2 6e+01)) "1.000000,1.000000,1.000000") "DontSpawnIfColliding" "MultiplyWithRoot" 0 0))))))))

(fn ConstructionScript)