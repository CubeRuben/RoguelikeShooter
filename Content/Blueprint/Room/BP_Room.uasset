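; BP_Room is a room actor that populates itself with BP_Pillar actors when play begins.
; On the authority only, the construction script picks a random Seed, and BeginPlay turns it into a random stream.
; It spawns a pillar at each PillarsSpawnOffsets entry relative to the room's location, then initializes each with its own number drawn from that stream.
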(event EventBeginPlay
  (Networking|SwitchHasAuthority
    (:Authority
      (Variables|Default|SetRandom%20Stream (Math|Random|MakeRandomStream (Variables|Default|GetSeed)))
      (for _array_element (Variables|Default|GetPillarsSpawnOffsets)
        (bind _returnvalue (Game|SpawnActorfromClass "/Game/Blueprint/Room/BP_Pillar.BP_Pillar_C" (Math|Transform|MakeTransform (+ _array_element (Transformation|GetActorLocation)) "0, 0, 0" "1.000000,1.000000,1.000000") "AlwaysSpawn" "MultiplyWithRoot" 0 0))
        (Default|Init _returnvalue (Class|KismetMathLibrary|RandomIntegerfromStream (Variables|Default|GetRandom%20Stream) 25000))))))

(fn ConstructionScript
  (Networking|SwitchHasAuthority
    (:Authority
      (Variables|Default|SetSeed (Math|Random|RandomInteger 2500)))))